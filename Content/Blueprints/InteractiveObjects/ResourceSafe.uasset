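; ResourceSafe is an interactive storage object where the player deposits carried resources.
; It caches the FirstPersonCharacterCustom on BeginPlay, and TriggerMainFunction adds that character's food, water, building materials, fuel and alien crystals to SafeInventory.
; It then clears the player's inventory and calls UpdateInventory on the character; the transfer is one-way, with no withdrawal logic here.
; Two getters supply its hover and description text.
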(event EventTriggerMainFunction
  (bind _asfirst_person_character_custom (Utilities|Casting|CastToFirstPersonCharacterCustom (Variables|Default|Getplayer)))
  (Variables|Default|SetSafeInventory (Utilities|Struct|MakeSimpleInventory (+ (.food (Variables|/Game/Imports/ThirdPersonBP/Blueprints/FirstPersonCharacterCustom.FirstPersonCharacterCustom_C|GetInventory _asfirst_person_character_custom)) (.food (Variables|Default|GetSafeInventory))) (+ (.water (Variables|/Game/Imports/ThirdPersonBP/Blueprints/FirstPersonCharacterCustom.FirstPersonCharacterCustom_C|GetInventory _asfirst_person_character_custom)) (.water (Variables|Default|GetSafeInventory))) (+ (.buildingmaterials (Variables|/Game/Imports/ThirdPersonBP/Blueprints/FirstPersonCharacterCustom.FirstPersonCharacterCustom_C|GetInventory _asfirst_person_character_custom)) (.buildingmaterials (Variables|Default|GetSafeInventory))) (+ (.fuel (Variables|Default|GetSafeInventory)) (.fuel (Variables|/Game/Imports/ThirdPersonBP/Blueprints/FirstPersonCharacterCustom.FirstPersonCharacterCustom_C|GetInventory _asfirst_person_character_custom))) (+ (.aliencrystal (Variables|/Game/Imports/ThirdPersonBP/Blueprints/FirstPersonCharacterCustom.FirstPersonCharacterCustom_C|GetInventory _asfirst_person_character_custom)) (.aliencrystal (Variables|Default|GetSafeInventory)))))
  (Variables|/Game/Imports/ThirdPersonBP/Blueprints/FirstPersonCharacterCustom.FirstPersonCharacterCustom_C|SetInventory _asfirst_person_character_custom "")
  (Default|UpdateInventory _asfirst_person_character_custom))

(event EventBeginPlay
  (bind _returnvalue (Actor|GetActorOfClass "/Game/Imports/ThirdPersonBP/Blueprints/FirstPersonCharacterCustom.FirstPersonCharacterCustom_C"))
  (Variables|Default|Setplayer _returnvalue))

(fn ConstructionScript)

(fn GetHoveronText
  (return (Variables|Interaction|GetOnHoverText)))

(fn GetObjectDescription
  (return (Variables|Interaction|GetOnPickupText)))
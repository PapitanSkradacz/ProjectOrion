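; Interactive key pickup that the player collects into their key inventory.
; When triggered, it casts the player reference to FirstPersonCharacterCustom, adds its unique key ID to that character's KeysIDinventory and destroys itself.
; Two getters supply its hover text and its description, the latter taken from the activation text.
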(event EventTriggerMainFunction
  (params (PlayerReference :type Actor%20Object%20Reference))
  (bind _asfirst_person_character_custom (Utilities|Casting|CastToFirstPersonCharacterCustom PlayerReference))
  (Utilities|Array|Add (Variables|/Game/Imports/ThirdPersonBP/Blueprints/FirstPersonCharacterCustom.FirstPersonCharacterCustom_C|GetKeysIDinventory _asfirst_person_character_custom) (Variables|Default|GetKeyUniqueID))
  (Actor|DestroyActor))

(fn ConstructionScript)

(fn GetHoveronText
  (return (Variables|Default|GetHoverOntext)))

(fn GetObjectDescription
  (return (Variables|Default|GetActivateText)))
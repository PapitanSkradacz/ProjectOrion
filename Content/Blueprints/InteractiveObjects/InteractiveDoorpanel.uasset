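; Interactive door panel that activates its referenced doors when triggered, optionally requiring a key.
; When a key is needed, it searches the player's key ID inventory for the required ID, then messages the doors, updates its description text and shows the open material.
; The front panel material starts closed or open according to the key requirement.
; Getter functions expose the hover and description texts.
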(event Custom|ChangeMatToOpen
  (Rendering|Material|SetMaterial (Variables|Default|GetFrontpanel) 0 "/Game/Materials/Debug/DoorpanelOpen.DoorpanelOpen"))

(event Custom|ChangeMatToClosed
  (Rendering|Material|SetMaterial (Variables|Default|GetFrontpanel) 0 "/Game/Materials/Debug/DoorpanelClosed.DoorpanelClosed"))

(event EventBeginPlay
  (if (Variables|Doorcontrol|GetIsKeyNeeded)
    (CallFunction|ChangeMattoClosed)
    (else
      (CallFunction|ChangeMattoOpen))))

(event EventTriggerMainFunction
  (params (PlayerReference :type Actor%20Object%20Reference))
  (if (Variables|Doorcontrol|GetIsKeyNeeded)
    (bind _asfirst_person_character_custom (Utilities|Casting|CastToFirstPersonCharacterCustom PlayerReference))
    (for _array_element (Variables|/Game/Imports/ThirdPersonBP/Blueprints/FirstPersonCharacterCustom.FirstPersonCharacterCustom_C|GetKeysIDinventory _asfirst_person_character_custom)
      (if (== _array_element (Variables|Doorcontrol|GetKeyIDrequired))
        (Variables|Doorcontrol|SetActivateText (Variables|Doorcontrol|GetTextAfterUsingKey))
        (Class|PuzzleFeatures|ActivateFunction(Message) (Variables|Doorcontrol|GetReferencedDoors))
        (CallFunction|ChangeMattoOpen)))
    (else
      (Class|PuzzleFeatures|ActivateFunction(Message) (Variables|Doorcontrol|GetReferencedDoors)))))

(fn ConstructionScript)

(fn GetHoveronText
  (return (Variables|Doorcontrol|GetHoverOnText)))

(fn GetObjectDescription
  (return (Variables|Doorcontrol|GetActivateText)))
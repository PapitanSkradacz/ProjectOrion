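; ActivatableButton is an interactable button that activates a referenced object, optionally only if the player holds a required key.
; TriggerMainFunction sends ActivateFunctionMessage to ReferencedObject1 directly, or first searches the FirstPersonCharacterCustom key inventory for a matching ID.
; A key match also swaps the activate text to its after-key version.
; Two getters supply the hover text and the current activate text as the object description.
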(event EventTriggerMainFunction
  (params (PlayerReference :type Actor%20Object%20Reference))
  (if (Variables|objectsinterface|GetKeyNeeded)
    (bind _asfirst_person_character_custom (Utilities|Casting|CastToFirstPersonCharacterCustom PlayerReference))
    (for _array_element (Variables|/Game/Imports/ThirdPersonBP/Blueprints/FirstPersonCharacterCustom.FirstPersonCharacterCustom_C|GetKeysIDinventory _asfirst_person_character_custom)
      (if (== _array_element (Variables|objectsinterface|GetKeyIDrequired))
        (Variables|objectsinterface|SetActivateText (Variables|objectsinterface|GetActivateTextAfterUsingKey))
        (Class|PuzzleFeatures|ActivateFunction(Message) (Variables|Default|GetReferencedObject1))))
    (else
      (Class|PuzzleFeatures|ActivateFunction(Message) (Variables|Default|GetReferencedObject1)))))

(fn ConstructionScript)

(fn GetHoveronText
  (return (Variables|objectsinterface|GetHoverOnText)))

(fn GetObjectDescription
  (return (Variables|objectsinterface|GetActivateText)))
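; Interactive two-sided door that toggles open and closed on activation and also reacts to BP_AiAlienWP overlapping its box.
; Separate open and close timelines move both door sides with additive local transforms, while IsWorking blocks activation during motion.
; A FlipFlop picks the direction, and a delay timeline re-triggers it to auto-close if still open.
; Alien begin and end overlaps play the timelines directly, bypassing that guard and toggle.
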(event OnComponentBeginOverlap(Box)
  (params (OverlappedComponent :type Primitive%20Component%20Object%20Reference) (OtherActor :type Actor%20Object%20Reference) (OtherComp :type Primitive%20Component%20Object%20Reference) (OtherBodyIndex :type Integer) (bFromSweep :type Boolean) (SweepResult :type Hit%20Result%20Structure%20%28by%20ref%29))
  (bind _doorsidea (Variables|Default|GetDoorSideA))
  (bind _doorsideb (Variables|Default|GetDoorSideB))
  (Utilities|Casting|CastToBP_AiAlienWP OtherActor)
  (bind _newtrack_0 (Timeline|DoorsOpeningTimeline PlayFromStart)
    (:Update
      (bind _result (Math|Float|NegateFloat _newtrack_0)
        (:%20%20
          (Class|SceneComponent|AddLocalTransform _doorsidea (Math|Transform|MakeTransform (Math|Vector|MakeVector 0.0 _result 0.0) "0, 0, 0" (.scale (Transformation|GetRelativeTransform _doorsidea))) false false)
          (Class|SceneComponent|AddLocalTransform _doorsideb (Math|Transform|MakeTransform (Math|Vector|MakeVector 0.0 _newtrack_0 0.0) "0, 0, 0" (.scale (Transformation|GetRelativeTransform _doorsideb))) false false))))
    (:Finished
      (Variables|Default|SetIsWorking false))))

(event OnComponentEndOverlap(Box)
  (params (OverlappedComponent :type Primitive%20Component%20Object%20Reference) (OtherActor :type Actor%20Object%20Reference) (OtherComp :type Primitive%20Component%20Object%20Reference) (OtherBodyIndex :type Integer))
  (bind _doorsidea (Variables|Default|GetDoorSideA))
  (bind _doorsideb (Variables|Default|GetDoorSideB))
  (Utilities|Casting|CastToBP_AiAlienWP OtherActor)
  (bind _newtrack_0 (Timeline|Timeline_0 PlayFromStart)
    (:Update
      (Class|SceneComponent|AddLocalTransform _doorsidea (Math|Transform|MakeTransform (Math|Vector|MakeVector 0.0 _newtrack_0 0.0) "0, 0, 0" (.scale (Transformation|GetRelativeTransform _doorsidea))) false false)
      (Class|SceneComponent|AddLocalTransform _doorsideb (Math|Transform|MakeTransform (Math|Vector|MakeVector 0.0 _newtrack_0 0.0) "0, 0, 0" (.scale (Transformation|GetRelativeTransform _doorsideb))) false false))
    (:Finished
      (Variables|Default|SetIsWorking false))))

(event Custom|OpenDoors
  (bind _doorsidea (Variables|Default|GetDoorSideA))
  (bind _doorsideb (Variables|Default|GetDoorSideB))
  (Variables|Default|SetIsWorking true)
  (bind _newtrack_0 (Timeline|DoorsOpeningTimeline PlayFromStart)
    (:Update
      (bind _result (Math|Float|NegateFloat _newtrack_0)
        (:%20%20
          (Class|SceneComponent|AddLocalTransform _doorsidea (Math|Transform|MakeTransform (Math|Vector|MakeVector 0.0 _result 0.0) "0, 0, 0" (.scale (Transformation|GetRelativeTransform _doorsidea))) false false)
          (Class|SceneComponent|AddLocalTransform _doorsideb (Math|Transform|MakeTransform (Math|Vector|MakeVector 0.0 _newtrack_0 0.0) "0, 0, 0" (.scale (Transformation|GetRelativeTransform _doorsideb))) false false))))
    (:Finished
      (Variables|Default|SetIsWorking false))))

(event Custom|CloseDoors
  (bind _doorsidea (Variables|Default|GetDoorSideA))
  (bind _doorsideb (Variables|Default|GetDoorSideB))
  (Variables|Default|SetIsWorking true)
  (bind _newtrack_0 (Timeline|Timeline_0 PlayFromStart)
    (:Update
      (Class|SceneComponent|AddLocalTransform _doorsidea (Math|Transform|MakeTransform (Math|Vector|MakeVector 0.0 _newtrack_0 0.0) "0, 0, 0" (.scale (Transformation|GetRelativeTransform _doorsidea))) false false)
      (Class|SceneComponent|AddLocalTransform _doorsideb (Math|Transform|MakeTransform (Math|Vector|MakeVector 0.0 _newtrack_0 0.0) "0, 0, 0" (.scale (Transformation|GetRelativeTransform _doorsideb))) false false))
    (:Finished
      (Variables|Default|SetIsWorking false))))

(event EventBeginPlay
  (Transformation|SetMobility (Variables|Default|GetSharedRoot) "Movable"))

(event EventActivateFunction
  (if (not (Variables|Default|GetIsWorking))
    (bind _isa (Utilities|FlowControl|FlipFlop :!label _label)
      (:A
        (CallFunction|OpenDoors)
        (Timeline|closeDoorsAfterTime PlayFromStart
          (:Finished
            (if _isa
              (goto _label)))))
      (:B
        (CallFunction|CloseDoors)))))

(fn ConstructionScript
  (Transformation|SetMobility (Variables|Default|GetSharedRoot) "Movable"))
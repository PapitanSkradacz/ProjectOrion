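; Interactive trigger object that starts a story and teleport sequence for the player.
; TriggerMainFunction casts the passed reference to FirstPersonCharacterCustom, blacks out the screen, hands over its StorytellingLines to display, and flags the character as awaiting teleportation.
; GetHoverOnText and GetObjectDescription return the trigger's hover and activation text.
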(event EventBeginPlay)

(event Collision|EventActorBeginOverlap
  (params (OtherActor :type Actor%20Object%20Reference)))

(event EventTick
  (params (DeltaSeconds :type Float%20%28single-precision%29)))

(event EventTriggerMainFunction
  (params (PlayerReference :type Actor%20Object%20Reference))
  (bind _asfirst_person_character_custom (Utilities|Casting|CastToFirstPersonCharacterCustom PlayerReference))
  (Default|UIBlackOutScreen _asfirst_person_character_custom)
  (Variables|/Game/Imports/ThirdPersonBP/Blueprints/FirstPersonCharacterCustom.FirstPersonCharacterCustom_C|SetStoryLines _asfirst_person_character_custom (Variables|Default|GetStorytellingLines))
  (Default|DisplayStoryLines _asfirst_person_character_custom)
  (Variables|/Game/Imports/ThirdPersonBP/Blueprints/FirstPersonCharacterCustom.FirstPersonCharacterCustom_C|SetTeleportationAwaiting _asfirst_person_character_custom true))

(fn ConstructionScript)

(fn GetHoveronText
  (return (Variables|Default|GetHoverOnText)))

(fn GetObjectDescription
  (return (Variables|Default|GetActivateText)))
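; Interactable resource pickup that adds a quantity of food, water, building materials, fuel or alien crystal to the player's inventory.
; BeginPlay sets a fixed rotation, then after a short delay caches the player character and picks the mesh from ResourceType.
; TriggerMainFunction adds Quantity if that resource is below its maximum, without clamping, and destroys the actor; otherwise it shows a "cannot carry more" message.
; Both outcomes refresh the inventory.
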(event EventBeginPlay
  (bind _pickupt1 (Variables|Default|GetPickupT1))
  (Transformation|SetActorRotation "0.000000, 0,90.000000")
  (Utilities|FlowControl|Delay 0.2)
  (bind _returnvalue (Actor|GetActorOfClass "/Game/Imports/ThirdPersonBP/Blueprints/FirstPersonCharacterCustom.FirstPersonCharacterCustom_C"))
  (Variables|Default|SetPlayer _returnvalue)
  (switch Utilities|FlowControl|Switch|SwitchonResourceTypes (Variables|ResourceScript|GetResourceType) ; Change the mesh
    (:NewEnumerator0
      (Components|StaticMesh|SetStaticMesh _pickupt1 "/Game/Scenes/Props/MREBags/MREBags.MREBags"))
    (:NewEnumerator1
      (Components|StaticMesh|SetStaticMesh _pickupt1 "/Game/Scenes/Props/WaterBag/WaterBag.WaterBag"))
    (:NewEnumerator2
      (Components|StaticMesh|SetStaticMesh _pickupt1 "/Game/Scenes/Props/ScrapMetal/ScrapMetal.ScrapMetal"))
    (:NewEnumerator3
      (Components|StaticMesh|SetStaticMesh _pickupt1 "/Game/Scenes/Props/Fuel/Fuel.Fuel"))
    (:NewEnumerator4
      (Components|StaticMesh|SetStaticMesh _pickupt1 "/Game/Scenes/Props/Plant/Plant.Plant"))))

(event EventTriggerMainFunction
  (params (PlayerReference :type Actor%20Object%20Reference))
  (bind _asfirst_person_character_custom (Utilities|Casting|CastToFirstPersonCharacterCustom (Variables|Default|GetPlayer)))
  (switch Utilities|FlowControl|Switch|SwitchonResourceTypes (Variables|ResourceScript|GetResourceType)
    (:NewEnumerator0
      (if (< (.food (Variables|/Game/Imports/ThirdPersonBP/Blueprints/FirstPersonCharacterCustom.FirstPersonCharacterCustom_C|GetInventory _asfirst_person_character_custom)) (.maxfood (Variables|/Game/Imports/ThirdPersonBP/Blueprints/FirstPersonCharacterCustom.FirstPersonCharacterCustom_C|GetMaxResourcesQuant _asfirst_person_character_custom)))
        (Utilities|Struct|SetmembersinSimpleInventory (Variables|/Game/Imports/ThirdPersonBP/Blueprints/FirstPersonCharacterCustom.FirstPersonCharacterCustom_C|GetInventory _asfirst_person_character_custom) (+ (.food (Variables|/Game/Imports/ThirdPersonBP/Blueprints/FirstPersonCharacterCustom.FirstPersonCharacterCustom_C|GetInventory _asfirst_person_character_custom)) (Variables|ResourceScript|GetQuantity)))
        (Default|UpdateInventory _asfirst_person_character_custom :!label _label)
        (Actor|DestroyActor)
        (else
          (Default|DisplayCustomMessage _asfirst_person_character_custom (Utilities|String|Append "You cannot carry more of: " (Utilities|String|EnumtoString (Variables|ResourceScript|GetResourceType)) "!") :!label _label_2)
          (Default|UpdateInventory _asfirst_person_character_custom))))
    (:NewEnumerator1
      (if (< (.water (Variables|/Game/Imports/ThirdPersonBP/Blueprints/FirstPersonCharacterCustom.FirstPersonCharacterCustom_C|GetInventory _asfirst_person_character_custom)) (.maxwater (Variables|/Game/Imports/ThirdPersonBP/Blueprints/FirstPersonCharacterCustom.FirstPersonCharacterCustom_C|GetMaxResourcesQuant _asfirst_person_character_custom)))
        (Utilities|Struct|SetmembersinSimpleInventory (Variables|/Game/Imports/ThirdPersonBP/Blueprints/FirstPersonCharacterCustom.FirstPersonCharacterCustom_C|GetInventory _asfirst_person_character_custom) (+ (.water (Variables|/Game/Imports/ThirdPersonBP/Blueprints/FirstPersonCharacterCustom.FirstPersonCharacterCustom_C|GetInventory _asfirst_person_character_custom)) (Variables|ResourceScript|GetQuantity)))
        (goto _label)
        (else
          (goto _label_2))))
    (:NewEnumerator2
      (if (< (.buildingmaterials (Variables|/Game/Imports/ThirdPersonBP/Blueprints/FirstPersonCharacterCustom.FirstPersonCharacterCustom_C|GetInventory _asfirst_person_character_custom)) (.maxbuildingmaterials (Variables|/Game/Imports/ThirdPersonBP/Blueprints/FirstPersonCharacterCustom.FirstPersonCharacterCustom_C|GetMaxResourcesQuant _asfirst_person_character_custom)))
        (Utilities|Struct|SetmembersinSimpleInventory (Variables|/Game/Imports/ThirdPersonBP/Blueprints/FirstPersonCharacterCustom.FirstPersonCharacterCustom_C|GetInventory _asfirst_person_character_custom) (+ (.buildingmaterials (Variables|/Game/Imports/ThirdPersonBP/Blueprints/FirstPersonCharacterCustom.FirstPersonCharacterCustom_C|GetInventory _asfirst_person_character_custom)) (Variables|ResourceScript|GetQuantity)))
        (goto _label)
        (else
          (goto _label_2))))
    (:NewEnumerator3
      (if (< (.fuel (Variables|/Game/Imports/ThirdPersonBP/Blueprints/FirstPersonCharacterCustom.FirstPersonCharacterCustom_C|GetInventory _asfirst_person_character_custom)) (.maxfuel (Variables|/Game/Imports/ThirdPersonBP/Blueprints/FirstPersonCharacterCustom.FirstPersonCharacterCustom_C|GetMaxResourcesQuant _asfirst_person_character_custom)))
        (Utilities|Struct|SetmembersinSimpleInventory (Variables|/Game/Imports/ThirdPersonBP/Blueprints/FirstPersonCharacterCustom.FirstPersonCharacterCustom_C|GetInventory _asfirst_person_character_custom) (+ (.fuel (Variables|/Game/Imports/ThirdPersonBP/Blueprints/FirstPersonCharacterCustom.FirstPersonCharacterCustom_C|GetInventory _asfirst_person_character_custom)) (Variables|ResourceScript|GetQuantity)))
        (goto _label)
        (else
          (goto _label_2))))
    (:NewEnumerator4
      (if (< (.aliencrystal (Variables|/Game/Imports/ThirdPersonBP/Blueprints/FirstPersonCharacterCustom.FirstPersonCharacterCustom_C|GetInventory _asfirst_person_character_custom)) (.maxcrystal (Variables|/Game/Imports/ThirdPersonBP/Blueprints/FirstPersonCharacterCustom.FirstPersonCharacterCustom_C|GetMaxResourcesQuant _asfirst_person_character_custom)))
        (Utilities|Struct|SetmembersinSimpleInventory (Variables|/Game/Imports/ThirdPersonBP/Blueprints/FirstPersonCharacterCustom.FirstPersonCharacterCustom_C|GetInventory _asfirst_person_character_custom) (+ (.aliencrystal (Variables|/Game/Imports/ThirdPersonBP/Blueprints/FirstPersonCharacterCustom.FirstPersonCharacterCustom_C|GetInventory _asfirst_person_character_custom)) (Variables|ResourceScript|GetQuantity)))
        (goto _label)
        (else
          (goto _label_2))))))

(fn ConstructionScript)

(fn GetHoveronText
  (return (Variables|ResourceScript|GetOnHoverText)))

(fn GetObjectDescription
  (return ""))
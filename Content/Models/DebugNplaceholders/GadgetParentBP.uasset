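; Parent Blueprint for gadgets (tools) that the first-person character can pick up and equip.
; TriggerMainFunction finds the character via GetActorOfClass, snaps the gadget to its WeaponSocket, then stores and equips it in the first free of three inventory slots, or shows a message when all are full.
; Enable and disable events toggle an enabled flag and visibility, while getter functions expose that state, hover text and an empty description.
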(event EventDisableGadget
  ;[1 1 1] Enable/disable gadget
  (Variables|Default|SetIsEnabled_0 false)
  (Rendering|SetActorHiddenInGame true))

(event EventEnableGadget
  ;[1 1 1] Enable/disable gadget
  (Variables|Default|SetIsEnabled_0 true)
  (Rendering|SetActorHiddenInGame false))

(event EventTriggerMainFunction
  ;[1 1 1] Pickup and equip
  (bind _returnvalue (Actor|GetActorOfClass "/Game/Imports/ThirdPersonBP/Blueprints/FirstPersonCharacterCustom.FirstPersonCharacterCustom_C"))
  (if (Utilities|IsValid (.GadgetSlot1 (Utilities|Struct|BreakSimpleInventory (Variables|/Game/Imports/ThirdPersonBP/Blueprints/FirstPersonCharacterCustom.FirstPersonCharacterCustom_C|GetInventory _returnvalue))))
    (if (Utilities|IsValid (.GadgetSlot2 (Utilities|Struct|BreakSimpleInventory (Variables|/Game/Imports/ThirdPersonBP/Blueprints/FirstPersonCharacterCustom.FirstPersonCharacterCustom_C|GetInventory _returnvalue))))
      (if (Utilities|IsValid (.GadgetSlot3 (Utilities|Struct|BreakSimpleInventory (Variables|/Game/Imports/ThirdPersonBP/Blueprints/FirstPersonCharacterCustom.FirstPersonCharacterCustom_C|GetInventory _returnvalue))))
        (Default|DisplayCustomMessage _returnvalue "You cannot hold more tools! All 3 slots are taken.")
        (else
          (Transformation|AttachComponentToComponent (Variables|/Game/Imports/ThirdPersonBP/Blueprints/FirstPersonCharacterCustom.FirstPersonCharacterCustom_C|GetWeaponSocket _returnvalue) "None" "SnapToTarget" "SnapToTarget" "KeepRelative" true)
          (Utilities|Struct|SetmembersinSimpleInventory (Variables|/Game/Imports/ThirdPersonBP/Blueprints/FirstPersonCharacterCustom.FirstPersonCharacterCustom_C|GetInventory _returnvalue) self)
          (Variables|/Game/Imports/ThirdPersonBP/Blueprints/FirstPersonCharacterCustom.FirstPersonCharacterCustom_C|SetSlot3Taken _returnvalue true)
          (Default|EquipSlot3 _returnvalue)))
      (else
        (Transformation|AttachComponentToComponent (Variables|/Game/Imports/ThirdPersonBP/Blueprints/FirstPersonCharacterCustom.FirstPersonCharacterCustom_C|GetWeaponSocket _returnvalue) "None" "SnapToTarget" "SnapToTarget" "KeepRelative" true)
        (Utilities|Struct|SetmembersinSimpleInventory (Variables|/Game/Imports/ThirdPersonBP/Blueprints/FirstPersonCharacterCustom.FirstPersonCharacterCustom_C|GetInventory _returnvalue) self)
        (Variables|/Game/Imports/ThirdPersonBP/Blueprints/FirstPersonCharacterCustom.FirstPersonCharacterCustom_C|SetSlot2Taken _returnvalue true)
        (Default|EquipSlot2 _returnvalue)))
    (else
      (Transformation|AttachComponentToComponent (Variables|/Game/Imports/ThirdPersonBP/Blueprints/FirstPersonCharacterCustom.FirstPersonCharacterCustom_C|GetWeaponSocket _returnvalue) "None" "SnapToTarget" "SnapToTarget" "KeepRelative" true)
      (Utilities|Struct|SetmembersinSimpleInventory (Variables|/Game/Imports/ThirdPersonBP/Blueprints/FirstPersonCharacterCustom.FirstPersonCharacterCustom_C|GetInventory _returnvalue) self)
      (Variables|/Game/Imports/ThirdPersonBP/Blueprints/FirstPersonCharacterCustom.FirstPersonCharacterCustom_C|SetSlot1Taken _returnvalue true)
      (Default|EquipSlot1 _returnvalue))))

(fn ConstructionScript)

(fn GetHoveronText
  (return (Variables|Default|GetHoverOnText)))

(fn GetObjectDescription
  (return ""))

(fn IsEnabled
  (if (Variables|Default|GetIsEnabled_0)
    (return true)
    (else
      (return false))))